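; Area measuring actor that lets the player outline a polygon with mouse clicks and reports its geographic coordinates; no area is calculated here.
; Tick traces under the cursor to stretch the latest cable and, from three points, a closing cable.
; Left click adds a point and cable, storing longitude/latitude/height via the default georeference.
; Right click stops drawing, removes the latest cable and sends each coordinate as JSON over Pixel Streaming.
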(event `is Colse`
  (params (is_close :type Boolean))
  (bind _points (`self.Points`))
  (bind (_location_x _location_y) (`KismetMathLibrary.BreakVector` (`self.Location`)))
  ;[1 1 1] 计算面积（应该没用）
  (`KismetArrayLibrary.Array_Clear` _points)
  (if true
    (for _ _points
      _)
    (`KismetArrayLibrary.Array_Add` (`self.Pointer 2d`) (`KismetMathLibrary.MakeVector2D` _location_x _location_y))))

(event `self.ReceiveTick`
  (params (DeltaSeconds :type "Float (single-precision)"))
  (bind _cabcle (`self.cabcle`))
  (bind (_worldlocation _worlddirection) (`PlayerController.DeprojectMousePositionToWorld` (`GameplayStatics.GetPlayerController` 0)))
  (if (`self.is Measure`)
    (bind _outhit (`KismetSystemLibrary.LineTraceSingle` :`Start` _worldlocation :`End` (* _worlddirection 2147483647) :`TraceChannel` "TraceTypeQuery1" :`DrawDebugType` "ForOneFrame"))
    (bind (_bblockinghit _binitialoverlap _time _distance _location) (`GameplayStatics.BreakHitResult` _outhit))
    (set `self.Location` _location)
    (`/Engine/EditorBlueprintResources/StandardMacros.IsValid` _cabcle
      (:`Is Valid`
        (bind _returnvalue (`KismetMathLibrary.InverseTransformLocation` (`self.GetTransform`) _location))
        (set `CableComponent.EndLocation` _returnvalue _cabcle)
        (if (>= (`KismetArrayLibrary.Array_Length` (`self.Points`)) 3)
          (if (`self.is close`)
            (set `CableComponent.EndLocation` _returnvalue (`self.close line`))
            (else
              (bind _returnvalue_2 (`AddComponent|NODE_AddCableComponent-3` :`RelativeTransform` (`KismetMathLibrary.MakeTransform` (`KismetMathLibrary.InverseTransformLocation` (`self.GetTransform`) (`|GetArrayItem` (`self.Points`))))))
              (bind _output_get (set `self.close line` _returnvalue_2))
              (set `CableComponent.EndLocation` _returnvalue _output_get)
              (set `self.is close` true))))))))

(event `click`
  (bind _location (`self.Location`))
  ;[1 1 1] 鼠标左键点击开始绘制
  (if (`self.is Measure`)
    (set `self.Location` _location)
    (bind _returnvalue (`AddComponent|NODE_AddCableComponent-0` :`RelativeTransform` (`KismetMathLibrary.MakeTransform` (`KismetMathLibrary.InverseTransformLocation` (`self.GetTransform`) _location))))
    (set `self.cabcle` _returnvalue)
    (`KismetArrayLibrary.Array_Add` (`self.Points`) _location)
    (bind _output_get (set `self.isclick` true))
    (if _output_get
      (bind _output_get_2 (set `self.clickpoint` (`.Location` (`GameplayStatics.BreakHitResult` (stale `self.ReceiveTick` _outhit)))))
      (bind _returnvalue_2 (`CesiumGeoreference.GetDefaultGeoreference`))
      (`KismetArrayLibrary.Array_Add` (`self.stringArray`) (`KismetStringLibrary.Conv_VectorToString` (`CesiumGeoreference.InaccurateTransformUnrealToLongitudeLatitudeHeight` _returnvalue_2 _output_get_2))))))

(event `right_click`
  (bind _cabcle (`self.cabcle`))
  ;[1 1 1] 鼠标右键点击停止绘制
  (set `self.is Measure` false)
  (set `self.is close` false)
  (`|ExecutionSequence`
    (:`then_0`
      (`/Engine/EditorBlueprintResources/StandardMacros.IsValid` _cabcle
        (:`Is Valid`
          (`ActorComponent.K2_DestroyComponent` _cabcle)
          (for _index (range (`KismetArrayLibrary.Array_Length` (`self.stringArray`)))
            (`PixelStreamerInputComponent.SendPixelStreamingResponse` (`self.GetComponentByClass` (`GameplayStatics.GetPlayerController` 0) "/Script/PixelStreaming.PixelStreamerInputComponent") (`BlueprintJsonLibrary.Conv_JsonObjectToString` (`BlueprintJsonLibrary.JsonMakeField` (`BlueprintJsonLibrary.JsonMake`) "coord" (`BlueprintJsonLibrary.JsonMakeString` (`|GetArrayItem` (`self.stringArray`) _index)))))))))))

(fn `UserConstructionScript`)