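; Clickable 3D text board for a Pixel Streaming scene that sends its board ID and data ID as JSON when its plane is clicked.
; Tick yaws the text from the camera look-at direction and scales the board by horizontal camera distance.
; Events set the text, fit plane width to its length, and change color by named material or parameter collection.
; saveMessage serializes the board's state into a JSON string.
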(event `self.Plane.OnClicked`
  (params (TouchedComponent :type "PrimitiveComponent Object Reference") (ButtonPressed :type "Key Structure"))
  (`PixelStreamerInputComponent.SendPixelStreamingResponse` (`self.GetComponentByClass` (`GameplayStatics.GetPlayerController` 0) "/Script/PixelStreaming.PixelStreamerInputComponent") (`BlueprintJsonLibrary.Conv_JsonObjectToString` (`BlueprintJsonLibrary.JsonMakeField` (`BlueprintJsonLibrary.JsonMakeField` (`BlueprintJsonLibrary.JsonMake`) "ID" (`BlueprintJsonLibrary.JsonMakeString` (`self.boardID`))) "dataID" (`BlueprintJsonLibrary.JsonMakeString` (`self.Descriptor`))))))

(event `change_text`
  (`Text3DComponent.SetText` (`self.Text3D`) (`self.content`)))

(event `change_size`
  (`SceneComponent.SetRelativeScale3D` (`self.Plane`) (`KismetMathLibrary.MakeVector` 1.0 (+ (* (`KismetStringLibrary.Len` (`KismetTextLibrary.Conv_TextToString` (`self.content`))) 0.66) 0.44) 4.0)))

(event `self.ReceiveTick`
  (params (DeltaSeconds :type "Float (single-precision)"))
  (bind _defaultsceneroot (`self.DefaultSceneRoot`))
  (bind _text3d (`self.Text3D`))
  ;[1 1 1] 设置朝向视口
  (`SceneComponent.K2_SetWorldRotation` _text3d (`KismetMathLibrary.MakeRotator` 0.0 0.0 (.yaw (`KismetMathLibrary.FindLookAtRotation` (`PlayerCameraManager.GetCameraLocation` (`GameplayStatics.GetPlayerCameraManager` 0)) (`SceneComponent.K2_GetComponentLocation` _text3d)))) false false)
  (`SceneComponent.SetWorldScale3D` _defaultsceneroot (`KismetMathLibrary.Conv_DoubleToVector` (/ (`KismetMathLibrary.Sqrt` (+ (`KismetMathLibrary.Square` (.x (- (`SceneComponent.K2_GetComponentLocation` _defaultsceneroot) (`PlayerCameraManager.GetCameraLocation` (`GameplayStatics.GetPlayerCameraManager` 0))))) (`KismetMathLibrary.Square` (.y (- (`SceneComponent.K2_GetComponentLocation` _defaultsceneroot) (`PlayerCameraManager.GetCameraLocation` (`GameplayStatics.GetPlayerCameraManager` 0))))))) 24000.0))))

(event `change_color`
  (`KismetMaterialLibrary.SetVectorParameterValue` "/Game/BP/color/freeColor/freeChangeColor.freeChangeColor" "freecolor" (`self.js2color`)))

(event `changeBasicColor`
  (bind _plane (`self.Plane`))
  (switch `string` (`self.basicColor`)
    (:`red`
      (`PrimitiveComponent.SetMaterial` _plane 0 "/Game/BP/color/basic/red.red"))
    (:`orange`
      (`PrimitiveComponent.SetMaterial` _plane 0 "/Game/BP/color/basic/orange.orange"))
    (:`yellow`
      (`PrimitiveComponent.SetMaterial` _plane 0 "/Game/BP/color/basic/yellow.yellow"))
    (:`green`
      (`PrimitiveComponent.SetMaterial` _plane 0 "/Game/BP/color/basic/green.green"))
    (:`cyan`
      (`PrimitiveComponent.SetMaterial` _plane 0 "/Game/BP/color/basic/cyan.cyan"))
    (:`blue`
      (`PrimitiveComponent.SetMaterial` _plane 0 "/Game/BP/color/basic/blue.blue"))
    (:`violet`
      (`PrimitiveComponent.SetMaterial` _plane 0 "/Game/BP/color/basic/violet.violet"))
    (:`black`
      (`PrimitiveComponent.SetMaterial` _plane 0 "/Game/BP/color/basic/black.black"))
    (:`white`
      (`PrimitiveComponent.SetMaterial` _plane 0 "/Game/BP/color/basic/white.white"))))

(event `saveMessage`
  (set `self.information` (`BlueprintJsonLibrary.Conv_JsonObjectToString` (`BlueprintJsonLibrary.JsonMakeField` (`BlueprintJsonLibrary.JsonMakeField` (`BlueprintJsonLibrary.JsonMakeField` (`BlueprintJsonLibrary.JsonMakeField` (`BlueprintJsonLibrary.JsonMakeField` (`BlueprintJsonLibrary.JsonMakeField` (`BlueprintJsonLibrary.JsonMake`) "ID" (`BlueprintJsonLibrary.JsonMakeString` (`self.boardID`))) "dataID" (`BlueprintJsonLibrary.JsonMakeString` (`self.Descriptor`))) "UI_content" (`BlueprintJsonLibrary.JsonMakeString` (`KismetTextLibrary.Conv_TextToString` (`self.content`)))) "setcolor" (`BlueprintJsonLibrary.JsonMakeString` (`KismetStringLibrary.Conv_ColorToString` (`self.js2color`)))) "Basiccolor" (`BlueprintJsonLibrary.JsonMakeString` (`self.basicColor`))) "Location" (`BlueprintJsonLibrary.JsonMakeString` (`KismetStringLibrary.Conv_VectorToString` (`self.boardLocation`)))))))

(fn `UserConstructionScript`)