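; Mouse-driven measuring tool that draws cable segments between clicked world points and reports their geographic coordinates; no distance is computed here.
; While measuring, Tick traces under the cursor and drags the newest cable's end to the hit.
; Each click adds a cable and stores the point as longitude/latitude/height via the default georeference.
; Right-click ends measuring, removes the dangling cable, and sends each stored coordinate as JSON through Pixel Streaming.
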(event `self.ReceiveTick`
  (params (DeltaSeconds :type "Float (single-precision)"))
  (bind _cabcle (`self.cabcle`))
  (bind (_worldlocation _worlddirection) (`PlayerController.DeprojectMousePositionToWorld` (`GameplayStatics.GetPlayerController` 0)))
  (if (`self.is measure`)
    (bind _outhit (`KismetSystemLibrary.LineTraceSingle` :`Start` _worldlocation :`End` (* _worlddirection 2147483647) :`TraceChannel` "TraceTypeQuery1" :`DrawDebugType` "ForOneFrame"))
    (bind (_bblockinghit _binitialoverlap _time _distance _location) (`GameplayStatics.BreakHitResult` _outhit))
    (set `self.Location` _location)
    (`/Engine/EditorBlueprintResources/StandardMacros.IsValid` _cabcle
      (:`Is Valid`
        (set `CableComponent.EndLocation` (`KismetMathLibrary.InverseTransformLocation` (`self.GetTransform`) _location) _cabcle)))))

(event `click`
  (bind _location (`self.Location`))
  ;[1 1 1] 鼠标左键点击开始绘制
  (if (`self.is measure`)
    (set `self.Location` _location)
    (bind _returnvalue (`AddComponent|NODE_AddCableComponent-0` :`RelativeTransform` (`KismetMathLibrary.MakeTransform` (`KismetMathLibrary.InverseTransformLocation` (`self.GetTransform`) _location))))
    (set `self.cabcle` _returnvalue)
    (bind _output_get (set `self.isclick` true))
    (if _output_get
      (bind _output_get_2 (set `self.clickpoint` (`.Location` (`GameplayStatics.BreakHitResult` (stale `self.ReceiveTick` _outhit)))))
      (bind _returnvalue_2 (`CesiumGeoreference.GetDefaultGeoreference`))
      (`KismetArrayLibrary.Array_Add` (`self.stringArray`) (`KismetStringLibrary.Conv_VectorToString` (`CesiumGeoreference.InaccurateTransformUnrealToLongitudeLatitudeHeight` _returnvalue_2 _output_get_2))))))

(event `right click`
  (bind _cabcle (`self.cabcle`))
  ;[1 1 1] 鼠标右键点击停止绘制
  (set `self.is measure` false)
  (`/Engine/EditorBlueprintResources/StandardMacros.IsValid` _cabcle
    (:`Is Valid`
      (`ActorComponent.K2_DestroyComponent` _cabcle)
      (for (_ _array_index) (`self.stringArray`)
        (`PixelStreamerInputComponent.SendPixelStreamingResponse` (`self.GetComponentByClass` (`GameplayStatics.GetPlayerController` 0) "/Script/PixelStreaming.PixelStreamerInputComponent") (`BlueprintJsonLibrary.Conv_JsonObjectToString` (`BlueprintJsonLibrary.JsonMakeField` (`BlueprintJsonLibrary.JsonMake`) "coord" (`BlueprintJsonLibrary.JsonMakeString` (`|GetArrayItem` (`self.stringArray`) _array_index)))))))))

(fn `UserConstructionScript`)