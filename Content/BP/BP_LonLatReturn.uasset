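; Pixel Streaming helper Blueprint that reports the longitude, latitude and height under the mouse cursor to the streaming client.
; While StartReturn is set, longLatReturn line-traces from the deprojected cursor with debug drawing and converts the hit through the default georeference.
; Each result is appended to a never-cleared array, and every stored entry is resent as "getLocation" JSON through PixelStreamerInputComponent.
; stopReturn clears the StartReturn flag.
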(event `longLatReturn`
  (bind (_worldlocation _worlddirection) (`PlayerController.DeprojectMousePositionToWorld` (`GameplayStatics.GetPlayerController` 0)))
  (if (`self.startReturn`)
    (bind _outhit (`KismetSystemLibrary.LineTraceSingle` :`Start` _worldlocation :`End` (* _worlddirection 2147483647) :`TraceChannel` "TraceTypeQuery1" :`DrawDebugType` "ForDuration" :`DrawTime` 2.0))
    (bind _returnvalue (`CesiumGeoreference.GetDefaultGeoreference`))
    (`KismetArrayLibrary.Array_Add` (`self.string`) (`KismetStringLibrary.Conv_VectorToString` (`CesiumGeoreference.InaccurateTransformUnrealToLongitudeLatitudeHeight` _returnvalue (`.Location` (`GameplayStatics.BreakHitResult` _outhit)))))
    (for (_ _array_index) (`self.string`)
      (`PixelStreamerInputComponent.SendPixelStreamingResponse` (`self.GetComponentByClass` (`GameplayStatics.GetPlayerController` 0) "/Script/PixelStreaming.PixelStreamerInputComponent") (`BlueprintJsonLibrary.Conv_JsonObjectToString` (`BlueprintJsonLibrary.JsonMakeField` (`BlueprintJsonLibrary.JsonMake`) "getLocation" (`BlueprintJsonLibrary.JsonMakeString` (`|GetArrayItem` (`self.string`) _array_index))))))))

(event `stopReturn`
  (set `self.startReturn` false))

(fn `UserConstructionScript`)